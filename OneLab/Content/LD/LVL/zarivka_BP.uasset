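; Fluorescent light fixture Blueprint (zarivka) with two configurable tube components, Trubice1 and Trubice2, for level dressing.
; The Construction Script sets each tube's visibility from its own boolean.
; A second boolean per tube swaps material slot 1 between the Emis and Emis2 materials.
; All logic runs at construction, as the Event Graph holds only disabled placeholder events.
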(event EventBeginPlay)

(event Collision|EventActorBeginOverlap
  (params (OtherActor :type Actor%20Object%20Reference)))

(event EventTick
  (params (DeltaSeconds :type Float%20%28single-precision%29)))

(fn ConstructionScript
  (bind _trubice2 (Variables|Default|Gettrubice2))
  (bind _trubice1 (Variables|Default|Gettrubice1))
  (Rendering|SetVisibility _trubice2 (Variables|trubice2|Gettrubice2_y/n) false)
  (Rendering|SetVisibility _trubice1 (Variables|trubice1|Gettrubice1%20y/n) false)
  (Utilities|FlowControl|Sequence
    (:then_0
      (if (Variables|trubice2|Gettrubice2%20emis%20on/off)
        (Rendering|Material|SetMaterial _trubice2 1 "/Game/LD/LVL/mat/emis.emis")
        (else
          (Rendering|Material|SetMaterial _trubice2 1 "/Game/LD/LVL/mat/emis2.emis2"))))
    (:then_1
      (if (Variables|trubice1|Gettrubice1%20emis%20on/off)
        (Rendering|Material|SetMaterial _trubice1 1 "/Game/LD/LVL/mat/emis.emis")
        (else
          (Rendering|Material|SetMaterial _trubice1 1 "/Game/LD/LVL/mat/emis2.emis2"))))))